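; BP_ShortRangeUnit is a player unit Blueprint that moves in response to axis input.
; MoveUnitForward and MoveUnitRight offset the actor along its local X and Y axes, scaled by MovementSpeed and world delta seconds for frame-rate-independent motion.
; The construction script only calls its parent version.
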(event Input|AxisEvents|InputAxisMoveUnitRight
  (params (AxisValue :type Float%20%28single-precision%29))
  (Transformation|AddActorLocalOffset (Math|Vector|MakeVector 0.0 (* AxisValue (Variables|Default|GetMovementSpeed) (Utilities|Time|GetWorldDeltaSeconds)) 0.0) false false))

(event Input|AxisEvents|InputAxisMoveUnitForward
  (params (AxisValue :type Float%20%28single-precision%29))
  (Transformation|AddActorLocalOffset (Math|Vector|MakeVector (* AxisValue (Variables|Default|GetMovementSpeed) (Utilities|Time|GetWorldDeltaSeconds)) 0.0 0.0) false false))

(fn ConstructionScript
  (|CallParentFunction))