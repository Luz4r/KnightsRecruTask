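; BP_PlayerUnit is a player unit that can be selected and has an attack range.
; The construction script scales an overlap mesh to the Range radius, and its begin/end overlaps only print attack start and stop messages.
; BeginPlay creates a dynamic material instance, which the Select event tints green when selected and white otherwise.
; Tick draws a debug cylinder showing the range.
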(event OnComponentEndOverlap(AttackRangeOverlapp)
  (params (OverlappedComponent :type Primitive%20Component%20Object%20Reference) (OtherActor :type Actor%20Object%20Reference) (OtherComp :type Primitive%20Component%20Object%20Reference) (OtherBodyIndex :type Integer))
  (Development|PrintString (Utilities|String|Append (Utilities|GetDisplayName self) " stopped attacking: " (Utilities|GetDisplayName OtherActor))))

(event OnComponentBeginOverlap(AttackRangeOverlapp)
  (params (OverlappedComponent :type Primitive%20Component%20Object%20Reference) (OtherActor :type Actor%20Object%20Reference) (OtherComp :type Primitive%20Component%20Object%20Reference) (OtherBodyIndex :type Integer) (bFromSweep :type Boolean) (SweepResult :type Hit%20Result%20Structure%20%28by%20ref%29))
  (Development|PrintString (Utilities|String|Append (Utilities|GetDisplayName self) " is attacking: " (Utilities|GetDisplayName OtherActor))))

(event EventBeginPlay
  (|CallParentFunction)
  (bind _returnvalue (Rendering|Material|CreateDynamicMaterialInstance (Variables|Default|GetRootStaticMesh) 0 "/Game/KnightsRecruTask/MaterialLibrary/MI_PlayerUnitColor.MI_PlayerUnitColor" "None" :!class /Script/Engine.PrimitiveComponent))
  (Variables|Internal|SetPlayerUnitColor _returnvalue))

(event EventTick
  (params (DeltaSeconds :type Float%20%28single-precision%29))
  (bind _returnvalue (Transformation|GetActorLocation))
  (|CallParentFunction DeltaSeconds)
  ;[1 1 1] Debug show unit attack range
  (Class|KismetSystemLibrary|DrawDebugCylinder _returnvalue _returnvalue (Variables|Default|GetRange) 24 "(R=0.000000,G=1.000000,B=0.000000,A=1.000000)" 0.0 0.0))

(event EventSelect
  (params (bSet :type Boolean))
  (CallFunction|SetSelectedUnit bSet))

(fn ConstructionScript
  (bind _range (Variables|Default|GetRange))
  (bind _returnvalue (/ _range 1e+02))
  (bind _returnvalue_2 (* _returnvalue 2.0))
  (|CallParentFunction)
  (Transformation|SetWorldScale3D (Variables|Default|GetAttackRangeOverlapp) (Math|Vector|MakeVector _returnvalue_2 _returnvalue_2 0.0)))

(fn SetSelectedUnit
  (params (bSet :type Boolean))
  (if bSet
    (Rendering|Material|SetVectorParameterValue (Variables|Internal|GetPlayerUnitColor) "Color" "(R=0.000000,G=1.000000,B=0.000000,A=1.000000)" :!class /Script/Engine.MaterialInstanceDynamic)
    (else
      (Rendering|Material|SetVectorParameterValue (Variables|Internal|GetPlayerUnitColor) "Color" "(R=1.000000,G=1.000000,B=1.000000,A=1.000000)" :!class /Script/Engine.MaterialInstanceDynamic))))