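; BP_PlayerUnitProjectile is a projectile for player units that flies in a set direction and disappears on contact.
; The construction script feeds InitialDirection into the projectile component's velocity and Speed into both its initial and maximum speed.
; Any overlap on the Sphere component destroys the actor; a comment mentions limiting this to "EnemyUnit", but the graph has no such check.
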(event OnComponentBeginOverlap(Sphere)
  (params (OverlappedComponent :type Primitive%20Component%20Object%20Reference) (OtherActor :type Actor%20Object%20Reference) (OtherComp :type Primitive%20Component%20Object%20Reference) (OtherBodyIndex :type Integer) (bFromSweep :type Boolean) (SweepResult :type Hit%20Result%20Structure%20%28by%20ref%29))
  ;[1 1 1] Only destroy when overlapping with "EnemyUnit"
  (Actor|DestroyActor))

(fn ConstructionScript
  (bind _projectilecomponent (Variables|Default|GetProjectileComponent))
  (|CallParentFunction)
  (Variables|/Script/Engine.MovementComponent|SetVelocity (Variables|Default|GetProjectileComponent) (Variables|Default|GetInitialDirection))
  (bind _output_get (Variables|/Script/Engine.ProjectileMovementComponent|SetInitialSpeed _projectilecomponent (Variables|Default|GetSpeed)))
  (Variables|/Script/Engine.ProjectileMovementComponent|SetMaxSpeed _projectilecomponent _output_get))