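; BP_AI is a player unit Blueprint that responds to selection and move commands.
; On BeginPlay it runs the parent logic and creates a dynamic material instance of MI_PlayerUnitColor on its static mesh.
; Select tints that material green when set and white when cleared.
; MovetoPosition passes the world location on through the OnMoveToRequested dispatcher, leaving the movement itself outside this graph.
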(event EventMovetoPosition
  (params (WorldLocation :type Vector :default "0, 0, 0"))
  (Default|CallOnMovetoRequested WorldLocation))

(event EventBeginPlay
  (|CallParentFunction)
  (bind _returnvalue (Rendering|Material|CreateDynamicMaterialInstance (Variables|Default|GetStaticMesh) 0 "/Game/KnightsRecruTask/MaterialLibrary/MI_PlayerUnitColor.MI_PlayerUnitColor" "None" :!class /Script/Engine.PrimitiveComponent))
  (Variables|Default|SetPlayerUnitColor _returnvalue))

(event EventSelect
  (params (bSet :type Boolean))
  (if bSet
    (Rendering|Material|SetVectorParameterValue (Variables|Default|GetPlayerUnitColor) "Color" "(R=0.000000,G=1.000000,B=0.000000,A=1.000000)" :!class /Script/Engine.MaterialInstanceDynamic)
    (else
      (Rendering|Material|SetVectorParameterValue (Variables|Default|GetPlayerUnitColor) "Color" "(R=1.000000,G=1.000000,B=1.000000,A=1.000000)" :!class /Script/Engine.MaterialInstanceDynamic))))

(fn ConstructionScript)