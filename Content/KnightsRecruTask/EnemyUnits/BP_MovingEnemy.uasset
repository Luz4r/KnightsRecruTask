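; BP_MovingEnemy is an enemy unit that chases whoever damages it and destroys itself on contact.
; DealDamage stores the damaging unit as Target and tells UnitMovement to move to it at MovementSpeed.
; Any overlap with its Sphere destroys the enemy, then sends the other actor a DealDamage message naming itself, with zero damage.
; The construction script only calls its parent's.
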(event OnComponentBeginOverlap(Sphere)
  (params (OverlappedComponent :type Primitive%20Component%20Object%20Reference) (OtherActor :type Actor%20Object%20Reference) (OtherComp :type Primitive%20Component%20Object%20Reference) (OtherBodyIndex :type Integer) (bFromSweep :type Boolean) (SweepResult :type Hit%20Result%20Structure%20%28by%20ref%29))
  (Actor|DestroyActor)
  (Class|BPIDamagable|DealDamage(Message) OtherActor self 0.0))

(event EventDealDamage
  (params (DamagingUnit :type Actor%20Object%20Reference) (DamageValue :type Float%20%28double-precision%29))
  (Variables|Internal|SetTarget DamagingUnit)
  (Class|UnitMovementComponent|MovetoActor (Variables|Default|GetUnitMovement) (Variables|Settings|GetMovementSpeed) (Variables|Internal|GetTarget)))

(fn ConstructionScript
  (|CallParentFunction))