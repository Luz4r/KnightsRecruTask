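; BP_PlayerStateMain is a player state Blueprint that keeps a list of the player's units and announces their destruction.
; On BeginPlay it gathers every actor implementing BPI_Selectable, binds to its OnDestroyed event and adds it to SpawnedPlayerUnits.
; DeleteDestroyedUnit removes a destroyed actor from that list and fires the OnUnitDestroyed dispatcher.
; Only actors present at BeginPlay are registered here.
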(event Custom|DeleteDestroyedUnit
  (params (DestroyedActor :type Actor%20Object%20Reference))
  (Utilities|Array|RemoveItem (Variables|Default|GetSpawnedPlayerUnits) DestroyedActor)
  (Default|CallOnUnitDestroyed DestroyedActor))

(event EventBeginPlay
  (|CallParentFunction)
  (bind _outactors (Actor|GetAllActorswithInterface "/Game/KnightsRecruTask/Core/BPI_Selectable.BPI_Selectable_C"))
  (for _array_element _outactors
    (Game|BindEventtoOnDestroyed _array_element (EventDispatchers|CreateEvent :!event Custom|DeleteDestroyedUnit))
    (Utilities|Array|Add (Variables|Default|GetSpawnedPlayerUnits) _array_element)))

(fn ConstructionScript)