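; RTS-style player controller that handles click and drag-box unit selection and move orders for the player's units.
; A short hold timer drives the selection box widget; releasing near the press point line-traces for a single BPI_Selectable actor.
; Drags trace both cursor ends into the world and select PlayerState's spawned units inside that flattened XY box.
; MoveUnit sends the traced point to selected units via interface message, with debug drawing.
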(event Custom|EnableSelectionBoxForMouseHold
  (Default|ShowSelectionBox (Variables|SelectionBox|GetSelectionBoxWidget) (Variables|SelectionBox|GetStartHoldMouseViewportPosition)))

(event EventBeginPlay
  (|CallParentFunction)
  (bind _returnvalue (UserInterface|CreateWidget "/Game/KnightsRecruTask/UI/WBP_SelectionBox.WBP_SelectionBox_C" self))
  (bind _output_get (Variables|SelectionBox|SetSelectionBoxWidget _returnvalue))
  (UserInterface|Viewport|AddtoViewport _output_get 0))

(event Input|ActionEvents|InputActionSelect
  (params (Key :type Key%20Structure :default "None"))
  (bind (_bavailable _tracestart _traceend) (CallFunction|GetMouseLocationforTrace))
  (bind (_worldlocation _worlddirection _returnvalue) (Game|Player|ConvertMouseLocationToWorldSpace))
  (bind (_bavailable_2 _tracestart_2 _traceend_2) (CallFunction|GetMouseLocationforTrace))
  (:Pressed
    (CallFunction|UnselectUnits)
    (if _returnvalue
      (Variables|SelectionBox|SetStartHoldMouseLocation _worldlocation)
      (Variables|SelectionBox|SetStartHoldMouseDirection _worlddirection)
      (bind _returnvalue_2 (Class|WidgetLayoutLibrary|GetMousePositiononViewport))
      (Variables|SelectionBox|SetStartHoldMouseViewportPosition _returnvalue_2)
      (bind _returnvalue_3 (Utilities|Time|SetTimerbyEvent (EventDispatchers|CreateEvent :!event Custom|EnableSelectionBoxForMouseHold) 0.07))
      (Variables|Internal|SetMouseHoldTimer _returnvalue_3)))
  (:Released
    (Utilities|Time|ClearandInvalidateTimerbyHandle (Variables|Internal|GetMouseHoldTimer))
    (Default|HideSelectionBox (Variables|SelectionBox|GetSelectionBoxWidget))
    (if (Utilities|Operators|EqualEqual (Variables|SelectionBox|GetStartHoldMouseLocation) (.WorldLocation (Game|Player|ConvertMouseLocationToWorldSpace)) 1.0)
      (if _bavailable
        (bind (_outhit _returnvalue_4) (Collision|LineTraceByChannel _tracestart _traceend "TraceTypeQuery3" false 0 "None" true "(R=1.000000,G=0.000000,B=0.000000,A=1.000000)" "(R=0.000000,G=1.000000,B=0.000000,A=1.000000)" 3.0))
        (if (and _returnvalue_4 (Utilities|DoesObjectImplementInterface (.HitActor (Collision|BreakHitResult _outhit)) "/Game/KnightsRecruTask/Core/BPI_Selectable.BPI_Selectable_C"))
          (Class|BPISelectable|Select(Message) (.HitActor (Collision|BreakHitResult _outhit)) true)
          (Utilities|Array|Add (Variables|Internal|GetSelectedUnits) (.HitActor (Collision|BreakHitResult _outhit)))))
      (elif _bavailable_2
        (bind _outhit_2 (Collision|LineTraceByChannel _tracestart_2 _traceend_2 "TraceTypeQuery1" false 0 "None" true "(R=1.000000,G=0.000000,B=0.000000,A=1.000000)" "(R=0.000000,G=1.000000,B=0.000000,A=1.000000)" 3.0))
        (bind _outhit_3 (Collision|LineTraceByChannel (Variables|SelectionBox|GetStartHoldMouseLocation) (+ (Variables|SelectionBox|GetStartHoldMouseLocation) (* (Variables|SelectionBox|GetStartHoldMouseDirection) 3e+03)) "TraceTypeQuery1" false 0 "None" true "(R=1.000000,G=0.000000,B=0.000000,A=1.000000)" "(R=0.000000,G=1.000000,B=0.000000,A=1.000000)" 3.0))
        (bind _spawnedplayerunits (CallFunction|GetSpawnedPlayerUnits))
        (for _array_element _spawnedplayerunits
          (if (Math|Geometry|IsPointinBox (Math|Vector|MakeVector (.X (Class|KismetMathLibrary|BreakVector3f (Transformation|GetActorLocation _array_element))) (.Y (Class|KismetMathLibrary|BreakVector3f (Transformation|GetActorLocation _array_element))) 0.0) (Math|Vector|Lerp(Vector) (Math|Vector|MakeVector (.X (Class|KismetMathLibrary|BreakVector3f (.Location (Collision|BreakHitResult _outhit_3)))) (.Y (Class|KismetMathLibrary|BreakVector3f (.Location (Collision|BreakHitResult _outhit_3)))) 0.0) (Math|Vector|MakeVector (.X (Class|KismetMathLibrary|BreakVector3f (.Location (Collision|BreakHitResult _outhit_2)))) (.Y (Class|KismetMathLibrary|BreakVector3f (.Location (Collision|BreakHitResult _outhit_2)))) 0.0) 0.5) (Math|Vector|MakeVector (|((abs((x1-x2)))/2) (.X (Class|KismetMathLibrary|BreakVector3f (.Location (Collision|BreakHitResult _outhit_3)))) (.X (Class|KismetMathLibrary|BreakVector3f (.Location (Collision|BreakHitResult _outhit_2))))) (|((abs((y1-y2)))/2) (.Y (Class|KismetMathLibrary|BreakVector3f (.Location (Collision|BreakHitResult _outhit_3)))) (.Y (Class|KismetMathLibrary|BreakVector3f (.Location (Collision|BreakHitResult _outhit_2))))) 0.0))
            (Class|BPISelectable|Select(Message) _array_element true)
            (Utilities|Array|Add (Variables|Internal|GetSelectedUnits) _array_element)))))))

(event Input|ActionEvents|InputActionMoveUnit
  (params (Key :type Key%20Structure :default "None"))
  (bind (_bavailable _tracestart _traceend) (CallFunction|GetMouseLocationforTrace))
  (:Pressed
    (Utilities|FlowControl|DoOnce false :!label _label
      (:Completed
        (if _bavailable
          (bind (_outhit _returnvalue) (Collision|LineTraceByChannel _tracestart _traceend "TraceTypeQuery3" false 0 "ForDuration" true "(R=1.000000,G=0.000000,B=0.000000,A=1.000000)" "(R=0.000000,G=1.000000,B=0.000000,A=1.000000)" 3.0))
          (if _returnvalue
            (Rendering|Debug|DrawDebugSphere (.Location (Collision|BreakHitResult _outhit)) 24.0 24 "(R=0.000000,G=0.000000,B=0.000000,A=1.000000)" 3.0 1.0)
            (for _array_element (Variables|Internal|GetSelectedUnits)
              (Class|BPISelectable|MovetoPosition(Message) _array_element (Math|Vector|MakeVector (.X (Class|KismetMathLibrary|BreakVector3f (.Location (Collision|BreakHitResult _outhit)))) (.Y (Class|KismetMathLibrary|BreakVector3f (.Location (Collision|BreakHitResult _outhit)))) 0.0))))))))
  (:Released
    (goto _label Reset)))

(fn ConstructionScript)

(fn UnselectUnits
  (for _array_element (Variables|Internal|GetSelectedUnits)
    (Class|BPISelectable|Select(Message) _array_element false))
  (Utilities|Array|Clear (Variables|Internal|GetSelectedUnits))
  (return))

(fn GetMouseLocationforTrace
  (bind (_worldlocation _worlddirection _returnvalue) (Game|Player|ConvertMouseLocationToWorldSpace))
  (return _returnvalue _worldlocation (+ _worldlocation (* _worlddirection 3e+03))))

(fn GetSpawnedPlayerUnits
  (bind _asbp_player_state_main (Utilities|Casting|CastToBP_PlayerStateMain (Variables|Default|GetPlayerState)))
  (return (Variables|/Game/KnightsRecruTask/Core/BP_PlayerStateMain.BP_PlayerStateMain_C|GetSpawnedPlayerUnits _asbp_player_state_main)))