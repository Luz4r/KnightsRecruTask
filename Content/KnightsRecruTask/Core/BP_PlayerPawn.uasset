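; Player pawn that acts as a movable camera, panned along the world X and Y axes by forward and right axis inputs.
; On BeginPlay it keeps its X and Y position and teleports to zero height.
; Each Tick, CameraMovement consumes pending input, normalizes it, scales by speed and delta time, and lerps toward it for eased acceleration.
; It applies the result as an unswept world offset, stopping instantly when input ends.
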(event EventBeginPlay
  (bind _returnvalue (Transformation|GetActorLocation))
  (|CallParentFunction)
  (Transformation|SetActorLocation (Math|Vector|MakeVector (.x _returnvalue) (.y _returnvalue) 0.0) false true))

(event EventTick
  (params (DeltaSeconds :type Float%20%28single-precision%29))
  (|CallParentFunction DeltaSeconds)
  (|CameraMovement DeltaSeconds))

(event Input|AxisEvents|InputAxisMovePlayerCameraForward
  (params (AxisValue :type Float%20%28single-precision%29))
  (Pawn|Input|AddMovementInput (Math|Vector|MakeVector AxisValue 0.0 0.0) 1.0 false))

(event Input|AxisEvents|InputAxisMovePlayerCameraRight
  (params (AxisValue :type Float%20%28single-precision%29))
  (Pawn|Input|AddMovementInput (Math|Vector|MakeVector 0.0 AxisValue 0.0) 1.0 false))

(fn ConstructionScript)